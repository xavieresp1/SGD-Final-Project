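; Single bowling pin actor that detects when it has been tipped over.
; Every Tick, it treats the Pin component's world roll and pitch as a 2D vector and compares its squared length to the squared TiltTolerance, ignoring yaw.
; The first time the tilt exceeds that tolerance, a DoOnce clears IsStanding, and nothing in this Blueprint sets it back.
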(event EventBeginPlay)

(event Collision|EventActorBeginOverlap
  (params (OtherActor :type Actor%20Object%20Reference)))

(event EventTick
  (params (DeltaSeconds :type Float%20%28single-precision%29))
  (bind _pin (Variables|Default|GetPin))
  (bind _returnvalue (Transformation|GetWorldRotation _pin))
  (bind (_roll _pitch) (Math|Rotator|BreakRotator _returnvalue))
  (if (> (Class|KismetMathLibrary|VSize2DSquared (Math|Vector2D|MakeVector2D _roll _pitch)) (Math|Float|Square (Variables|Default|GetTiltTolerance)))
    (Utilities|FlowControl|DoOnce false
      (:Completed
        (Variables|Default|SetIsStanding false)))))

(fn ConstructionScript)