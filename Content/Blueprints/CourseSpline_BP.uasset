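; CourseSpline_BP is a spline-driven actor that builds a course out of repeated spline mesh pieces in its construction script.
; It divides the spline into whole sections sized by the actor's Y scale, leaving any shorter remainder at the end uncovered.
; Each section becomes a Y-forward, collision-enabled spline mesh, with tangents clamped to the section length to prevent stretching.
; The event graph has no runtime logic.
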(event EventBeginPlay)

(event Collision|EventActorBeginOverlap
  (params (OtherActor :type Actor%20Object%20Reference)))

(event EventTick
  (params (DeltaSeconds :type Float%20%28single-precision%29)))

(fn ConstructionScript
  (bind _spline (Variables|Default|GetSpline))
  ;[1 1 1] Spline Functionality
  (Variables|Default|SetSection%20Length (* 1e+02 (.y (Transformation|GetActorScale3D))))
  (for _index (range 0 (- (Math|Float|Truncate (/ (Spline|GetSplineLength (Variables|Default|GetSpline)) (Variables|Default|GetSection%20Length))) 1))
    (bind _returnvalue (AddComponent|AddSplineMeshComponent false))
    (SplineMesh|SetForwardAxis _returnvalue "Y" true)
    (Collision|SetCollisionEnabled _returnvalue "QueryAndPhysics")
    (SplineMesh|SetStartandEnd _returnvalue (Spline|GetLocationatDistanceAlongSpline _spline (* _index (Variables|Default|GetSection%20Length)) "Local") (Math|Vector|ClampVectorSize (Spline|GetTangentatDistanceAlongSpline _spline (* _index (Variables|Default|GetSection%20Length)) "Local") 0.0 (Variables|Default|GetSection%20Length)) (Spline|GetLocationatDistanceAlongSpline _spline (* (+ _index 1) (Variables|Default|GetSection%20Length)) "Local") (Math|Vector|ClampVectorSize (Spline|GetTangentatDistanceAlongSpline _spline (* (+ _index 1) (Variables|Default|GetSection%20Length)) "Local") 0.0 (Variables|Default|GetSection%20Length)) true :!class /Script/Engine.SplineMeshComponent)))