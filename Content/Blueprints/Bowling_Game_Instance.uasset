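; Bowling game instance that keeps per-frame scores, frame count and throws while each frame loads its own level.
; ScoreForFrame reads the score from the pins actor, records the throw and flags strikes or spares, then recomputes bonuses.
; UpdateAllScores fills each strike or spare bonus from following frames, including consecutive strikes.
; The score widget, created on Init, then appears with UI-only input; NextFrame and ResetLevel handle level changes.
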(event EventInit
  (bind _returnvalue (UserInterface|CreateWidget "/Game/Widgets/ScoreUI.ScoreUI_C"))
  (Variables|Default|SetScoreUI _returnvalue))

(fn ScoreforFrame
  (bind _returnvalue (Game|GetPlayerController 0))
  (bind _framescores (Variables|Default|GetFrameScores))
  (bind _frame (Variables|Default|GetFrame))
  (bind _scoreui (Variables|Default|GetScoreUI))
  (bind _returnvalue_2 (- _frame 1))
  (bind _output (Utilities|Array|Get(acopy) _framescores _returnvalue_2))
  (bind (_score1 _score2 _additscore _isstrike _isspare) (Utilities|Struct|BreakFrame _output))
  (bind _outactors (Actor|GetAllActorsOfClass "/Game/Blueprints/Bowling_Pins_Blueprint.Bowling_Pins_Blueprint_C"))
  (bind _score (Default|CalculateScore (Utilities|Array|Get(acopy) _outactors)))
  (if (== (Variables|Default|GetThrows) 1)
    (bind _structout (Utilities|Struct|SetmembersinFrame _output _score _score2 _additscore _isstrike _isspare))
    (if (== (.Score1 (Utilities|Struct|BreakFrame _structout)) 10)
      (Utilities|Struct|SetmembersinFrame _structout (.Score1 (Utilities|Struct|BreakFrame _structout)) (.Score2 (Utilities|Struct|BreakFrame _structout)) (.AdditScore (Utilities|Struct|BreakFrame _structout)) true false))
    (else
      (bind _structout_2 (Utilities|Struct|SetmembersinFrame _output _score1 _score _additscore _isstrike _isspare))
      (if (== (+ (.Score1 (Utilities|Struct|BreakFrame _structout_2)) (.Score2 (Utilities|Struct|BreakFrame _structout_2))) 10)
        (Utilities|Struct|SetmembersinFrame _structout_2 (.Score1 (Utilities|Struct|BreakFrame _structout_2)) (.Score2 (Utilities|Struct|BreakFrame _structout_2)) (.AdditScore (Utilities|Struct|BreakFrame _structout_2)) false true))))
  (CallFunction|UpdateAllScores)
  (Default|Refresh _scoreui)
  (UserInterface|Viewport|AddtoViewport _scoreui 0)
  (Widget|SetVisibility _scoreui "Visible")
  (Variables|/Script/Engine.PlayerController|SetbShowMouseCursor _returnvalue true)
  (Input|SetInputModeUIOnly _returnvalue _scoreui "LockAlways"))

(fn UpdateAllScores
  (for (_array_element _array_index) (Variables|Default|GetFrameScores)
    (if (.IsStrike (Utilities|Struct|BreakFrame _array_element)) ; Is this frame a strike?
      ;[1 1 1] Is next frame a strike?
      (if (.IsStrike (Utilities|Struct|BreakFrame (Utilities|Array|Get(acopy) (Variables|Default|GetFrameScores) (+ _array_index 1))))
        ;[1 1 1] Next frame is ALSO a strike
        (Utilities|Struct|SetmembersinFrame _array_element (.Score1 (Utilities|Struct|BreakFrame _array_element)) (.Score2 (Utilities|Struct|BreakFrame _array_element)) (+ (.Score1 (Utilities|Struct|BreakFrame (Utilities|Array|Get(acopy) (Variables|Default|GetFrameScores) (+ _array_index 2)))) (.Score1 (Utilities|Struct|BreakFrame (Utilities|Array|Get(acopy) (Variables|Default|GetFrameScores) (+ _array_index 1))))) (.IsStrike (Utilities|Struct|BreakFrame _array_element)) (.IsSpare (Utilities|Struct|BreakFrame _array_element)))
        (else
          ;[1 1 1] Next frame is NOT a strike
          (Utilities|Struct|SetmembersinFrame _array_element (.Score1 (Utilities|Struct|BreakFrame _array_element)) (.Score2 (Utilities|Struct|BreakFrame _array_element)) (+ (.Score1 (Utilities|Struct|BreakFrame (Utilities|Array|Get(acopy) (Variables|Default|GetFrameScores) (+ _array_index 1)))) (.Score2 (Utilities|Struct|BreakFrame (Utilities|Array|Get(acopy) (Variables|Default|GetFrameScores) (+ _array_index 1))))) (.IsStrike (Utilities|Struct|BreakFrame _array_element)) (.IsSpare (Utilities|Struct|BreakFrame _array_element)))))
      (elif (.IsSpare (Utilities|Struct|BreakFrame _array_element)) ; Is this frame a spare?
        (|SetBy-RefVar _array_element (Utilities|Struct|MakeFrame (.Score1 (Utilities|Struct|BreakFrame _array_element)) (.Score2 (Utilities|Struct|BreakFrame _array_element)) (.Score1 (Utilities|Struct|BreakFrame (Utilities|Array|Get(acopy) (Variables|Default|GetFrameScores) (+ _array_index 1)))) (.IsStrike (Utilities|Struct|BreakFrame _array_element)) (.IsSpare (Utilities|Struct|BreakFrame _array_element))))))))

(fn ResetLevel
  (Default|CallRestartLevel))

(fn NextFrame
  (bind _frame (Variables|Default|GetFrame))
  (bind _output_get (LocalVariables|SetNext%20Level%20Name (Utilities|Array|Get(acopy) (Variables|Default|GetFrameLevels) _frame)))
  (Math|Integer|IncrementInt _frame
    (:%20%20
      (Variables|Default|SetThrows 0)
      (Game|OpenLevel(byName) _output_get))))