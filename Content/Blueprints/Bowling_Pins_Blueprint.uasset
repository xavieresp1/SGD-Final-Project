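; Bowling pin rack actor that spawns and tracks the pins for a bowling game.
; On BeginPlay it spawns a Single_Bowling_Pin at each child component of its scene root and stores them in Pins.
; CalculateScore returns PinsOver, which increments for pins still standing despite its name.
; CleanUpFallenPins records fallen indices, then loops backward removing entries and calling DestroyActor, but tests only for index 0 rather than the current one.
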(event EventBeginPlay
  (for _array_element (Components|GetChildrenComponents (Variables|Default|GetDefaultSceneRoot) false)
    (bind _returnvalue (Game|SpawnActorfromClass "/Game/Blueprints/Single_Bowling_Pin.Single_Bowling_Pin_C" (Math|Transform|MakeTransform (.Location (Math|Transform|BreakTransform (Transformation|GetWorldTransform _array_element))) (.Rotation (Math|Transform|BreakTransform (Transformation|GetWorldTransform _array_element)))) "Undefined" 0 0))
    (Utilities|Array|Add (Variables|Default|GetPins) _returnvalue)))

(fn ConstructionScript)

(fn CalculateScore
  (for _array_element (Variables|Default|GetPins)
    (if (Variables|/Game/Blueprints/Single_Bowling_Pin.Single_Bowling_Pin_C|GetIsStanding _array_element)
      (Math|Integer|IncrementInt (LocalVariables|GetPinsOver))))
  (return (LocalVariables|GetPinsOver)))

(fn CleanUpFallenPins
  (bind _pins (Variables|Default|GetPins))
  (for (_array_element _array_index) _pins
    (if (not (Variables|/Game/Blueprints/Single_Bowling_Pin.Single_Bowling_Pin_C|GetIsStanding _array_element))
      (Utilities|Array|Add (LocalVariables|GetCleanupIndices) _array_index)))
  (for _index (range (- (Utilities|Array|Length _pins) 1) 0)
    (if (Utilities|Array|ContainsItem (LocalVariables|GetCleanupIndices) 0)
      (Utilities|Array|RemoveIndex (Variables|Default|GetPins) _index)
      (Actor|DestroyActor))))