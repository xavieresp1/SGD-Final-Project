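; Draft spline actor, apparently for a course lane, whose construction script is empty; every placement graph is disconnected and never runs.
; Unwired experiments either space PlacedMesh instances by bounding-box length plus Offset, or add spline mesh segments with tangents clamped to section length.
; Instance locations convert a point-distance scalar to a vector instead of sampling spline positions.
; The spline mesh components never get PlacedMesh assigned in these graphs.
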(fn ConstructionScript)